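; BP_Hoverable is a component that highlights its owning actor while the mouse cursor is over it.
; On BeginPlay it binds to the owner's begin and end cursor-over events and caches the owner's skeletal mesh component.
; The handlers track the hover state and swap the mesh's first material to solid blue, then to a hard-coded hex material on exit rather than the original one.
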(event Custom|Begin%20Cursor%20Over
  (params (TouchedActor :type Actor%20Object%20Reference))
  (bind _output_get (Variables|Default|SetIsCursorOn true))
  (Utilities|IsValid (Variables|Default|GetMesh)
    (:Is%20Valid
      (if _output_get
        (Rendering|Material|SetMaterial (Variables|Default|GetMesh) 0 "/Game/LevelPrototyping/Materials/MI_Solid_Blue.MI_Solid_Blue")))))

(event Custom|EndCursorOver
  (params (TouchedActor :type Actor%20Object%20Reference))
  (bind _output_get (Variables|Default|SetIsCursorOn false))
  (Utilities|IsValid (Variables|Default|GetMesh)
    (:Is%20Valid
      (if (not _output_get)
        (Rendering|Material|SetMaterial (Variables|Default|GetMesh) 0 "/Game/Assetts/Art/bMat_Hex_v1_001.bMat_Hex_v1_001")))))

(event EventBeginPlay
  (bind _returnvalue (Components|GetOwner))
  (bind _returnvalue_2 (Components|GetOwner))
  (bind _returnvalue_3 (Actor|GetComponentbyClass _returnvalue "/Script/Engine.SkeletalMeshComponent"))
  (bind _returnvalue_4 (Actor|GetComponentbyClass _returnvalue_2 "/Script/Engine.SkeletalMeshComponent"))
  (Utilities|FlowControl|Sequence
    (:then_0
      (EventDispatchers|BindEventtoOnBeginCursorOver _returnvalue_2 (delegate Custom|Begin%20Cursor%20Over))
      (Utilities|IsValid _returnvalue_4
        (:Is%20Valid
          (Variables|Default|SetMesh _returnvalue_4))))
    (:then_1
      (EventDispatchers|BindEventtoOnEndCursorOver _returnvalue (delegate Custom|EndCursorOver))
      (Utilities|IsValid _returnvalue_3
        (:Is%20Valid
          (Variables|Default|SetMesh _returnvalue_3))))))