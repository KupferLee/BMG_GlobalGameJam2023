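; Base hex tile for a turn-based root-spreading game, where clicking a tile next to a rooted one roots it.
; On BeginPlay, Mapping links six neighbors via directional hitbox overlaps against all tiles, then click is bound.
; A click on a rootable, affordable tile with rooted neighbors charges the tree controller, adds tile value, advances the turn and plays an animation once.
; The cost-widget hover binding never runs.
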(event Custom|CustomEvent
  (params (TouchedActor :type Actor%20Object%20Reference) (ButtonPressed :type Key%20Structure :default "None"))
  (if (Variables|Default|GetIsRootable)
    (|CheckHowManyneighborsAreRooted
      (:true
        (if (> (Variables|Default|GetRootedNeighborCount) 0)
          ;[1 1 1] check if value < currency
          (bind _asbp_tree_controller (Utilities|Casting|CastToBP_TreeController (Game|GetPlayerController 0)))
          (bind _output_get (Variables|Default|SetRef_TreeController _asbp_tree_controller))
          (if (<= (Variables|Default|GetRootCosts) (Variables|/Game/Blueprints/BP_TreeController.BP_TreeController_C|GetCurrency _output_get))
            ;[1 1 1] decrease currency depending on tile value
            (Utilities|FlowControl|DoOnce false
              (:Completed
                (Variables|/Game/Blueprints/BP_TreeController.BP_TreeController_C|SetCurrency (Variables|Default|GetRef_TreeController) (- (Variables|/Game/Blueprints/BP_TreeController.BP_TreeController_C|GetCurrency (Variables|Default|GetRef_TreeController)) (Variables|Default|GetRootCosts)))
                ;[1 1 1] add currency if tile has value
                (Variables|/Game/Blueprints/BP_TreeController.BP_TreeController_C|SetCurrency (Variables|Default|GetRef_TreeController) (+ (Variables|/Game/Blueprints/BP_TreeController.BP_TreeController_C|GetCurrency (Variables|Default|GetRef_TreeController)) (Variables|Default|GetTileValue)))
                ;[1 1 1] increase turn count with every click 1
                (Variables|/Game/Blueprints/BP_TreeController.BP_TreeController_C|SetCurrent%20Turn (Variables|Default|GetRef_TreeController) (+ (Variables|/Game/Blueprints/BP_TreeController.BP_TreeController_C|GetCurrent%20Turn (Variables|Default|GetRef_TreeController)) 1))
                ;[1 1 1] play flip animation
                (Components|Animation|PlayAnimation (Variables|Default|GetSkeletalMesh) (Variables|Default|GetAnimationSequence) false)
                (Variables|Default|SetIsRooted true)))))))))

(event Custom|OnBeginCursorOver_Event
  (params (TouchedActor :type Actor%20Object%20Reference))
  (bind _returnvalue (UserInterface|CreateWidget "/Game/Blueprints/UI_Widgets/W_HUD.W_HUD_C"))
  (Variables|/Game/Blueprints/UI_Widgets/W_HUD.W_HUD_C|SetCurrent%20Tile%20Costs _returnvalue (Variables|Default|GetRootCosts)))

(event EventBeginPlay
  (|Mapping
    (:then_6
      (EventDispatchers|BindEventtoOnClicked (delegate Custom|CustomEvent)))))

(fn ConstructionScript)

(fn NewFunction
  (params (Array :type Array%20of%20BP%20Tile%20Base%20Object%20References) (Target :type Primitive%20Component%20Object%20Reference)))