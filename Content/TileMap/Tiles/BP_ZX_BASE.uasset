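; BP_ZX_BASE is a tile map tile that counts as a found temple once it is rooted.
; It sets its root cost on BeginPlay and calls HoverCosts when the cursor moves over its skeletal mesh.
; A looping timer, used in place of the disabled Tick, polls IsRooted at roughly frame rate and increments TemplesFound on BP_TreeController once through a DoOnce.
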(event OnBeginCursorOver(SkeletalMesh)
  (params (TouchedComponent :type Primitive%20Component%20Object%20Reference))
  (CallFunction|HoverCosts))

(event Custom|Initialize%20IsRooted%20Loop
  (Utilities|Time|SetTimerbyEvent (delegate Custom|Check%20If%20Rooted) 0.0167 true))

(event Custom|Check%20If%20Rooted
  (if (Variables|Default|GetIsRooted)
    (Utilities|FlowControl|DoOnce false
      (:Completed
        (bind _asbp_tree_controller (Utilities|Casting|CastToBP_TreeController (Game|GetPlayerController 0)))
        (Variables|/Game/Blueprints/BP_TreeController.BP_TreeController_C|SetTemples%20Found _asbp_tree_controller (+ (Variables|/Game/Blueprints/BP_TreeController.BP_TreeController_C|GetTemples%20Found _asbp_tree_controller) 1))))))

(event EventBeginPlay
  (Variables|Default|SetRootCosts 3)
  (CallFunction|InitializeIsRootedLoop)
  (|CallParentFunction))

(event Collision|EventActorBeginOverlap
  (params (OtherActor :type Actor%20Object%20Reference)))

(event EventTick
  (params (DeltaSeconds :type Float%20%28single-precision%29))
  (|CallParentFunction DeltaSeconds) ; This node is disabled and will not be called.\nDrag off pins to build functionality.
)

(fn ConstructionScript
  (|CallParentFunction))