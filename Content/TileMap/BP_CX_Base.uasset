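; BP_CX_Base is a base tile actor for a tile map that discovers its six neighbors, in a layout consistent with a hex grid.
; On BeginPlay, Mapping waits briefly, then loops over all other BP_CX_Base actors.
; Each directional hitbox (N, NE, NW, S, SE, SW) is overlap-tested against their TileHitbox, storing matches as neighbor references.
; Tick, the construction script and NewFunction do no useful work.
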(event EventBeginPlay
  (|Mapping))

(event EventTick
  (params (DeltaSeconds :type Float%20%28single-precision%29)))

(fn ConstructionScript)

(fn NewFunction
  (params (Array :type Array%20of%20BP%20CX%20Base%20Object%20References) (Target :type Primitive%20Component%20Object%20Reference))
  (for _array_element Array
    (if (Class|PrimitiveComponent|IsOverlappingComponent Target)
      _)))