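; Base tile for a six-neighbour (hex-style) tile map where clicking spreads roots from tile to tile.
; After a short BeginPlay delay, the Mapping macro finds neighbours by testing six directional hitboxes against every other tile's hitbox, then binds the click event.
; Clicking a rootable tile counts its rooted neighbours.
; If any exist, the tile plays its skeletal mesh animation once and becomes rooted.
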(event Custom|CustomEvent
  (params (TouchedActor :type Actor%20Object%20Reference) (ButtonPressed :type Key%20Structure :default "None"))
  (if (Variables|Default|GetIsRootable)
    (|CheckHowManyneighborsAreRooted
      (:true
        (if (> (Variables|Default|GetRootedNeighborCount) 0)
          (Utilities|FlowControl|DoOnce false
            (:Completed
              (Components|Animation|PlayAnimation (Variables|Default|GetSkeletalMesh) (Variables|Default|GetAnimationSequence) false)
              (Variables|Default|SetIsRooted true))))))))

(event EventBeginPlay
  (|Mapping
    (:then_6
      (EventDispatchers|BindEventtoOnClicked (delegate Custom|CustomEvent)))))

(event EventTick
  (params (DeltaSeconds :type Float%20%28single-precision%29)))

(fn ConstructionScript)

(fn NewFunction
  (params (Array :type Array%20of%20BP%20Tile%20Base%20Object%20References) (Target :type Primitive%20Component%20Object%20Reference)))