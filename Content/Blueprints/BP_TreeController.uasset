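; Player controller that runs the game flow from main menu and loading screen to HUD, story textboxes, pause menu and end screens.
; It moves the pawn as a camera through MoveCam, using screen-edge panning, axis input and height-limited zoom.
; Looping timers check currency for a loss, temples found for a win, and the first temple for a textbox.
; Debug-style inputs add currency and open a textbox.
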(event Custom|CreditButtonClicked
  ;[1 1 1] Credit Screen
  (bind _returnvalue (UserInterface|CreateWidget "/Game/Blueprints/UI_Widgets/W_CreditsScreen.W_CreditsScreen_C"))
  (UserInterface|Viewport|AddtoViewport _returnvalue 0))

(event Custom|Play%20Button%20Clicked
  ;[1 1 1] Start Game with Loading Screen & Delay
  (Viewport|RemoveAllWidgets)
  (Input|SetInputModeGameOnly (Game|GetPlayerController 0) false)
  (Game|SetGamePaused false)
  (bind _returnvalue (UserInterface|CreateWidget "/Game/Blueprints/UI_Widgets/W_Loading_Screen.W_Loading_Screen_C"))
  (UserInterface|Viewport|AddtoViewport _returnvalue 0)
  (Utilities|FlowControl|Delay (Variables|Default|GetLoading%20Screen%20Delay))
  (Viewport|RemoveAllWidgets)
  (Input|SetInputModeGameOnly 0 false)
  (bind _returnvalue_2 (UserInterface|CreateWidget "/Game/Blueprints/UI_Widgets/W_HUD.W_HUD_C"))
  (bind _output_get (Variables|Default|SetRef_Hud _returnvalue_2))
  (UserInterface|Viewport|AddtoViewport _output_get 0)
  (Variables|Default|SetCurrent%20Text (Variables|Default|GetStory%20Dump%20Text))
  (CallFunction|OpenTextbox)
  (CallFunction|InitializeLooseWinLoop)
  (CallFunction|InitializeCheckingTutorialTemple))

(event Custom|Coninue%20Game
  ;[1 1 1] continue game from pause screen
  (Widget|RemovefromParent (Variables|Default|GetRef_PauseScreen))
  (Input|SetInputModeGameOnly (Game|GetPlayerController 0) false)
  (Variables|/Script/Engine.PlayerController|SetbShowMouseCursor (Game|GetPlayerController 0) false)
  (Game|SetGamePaused false))

(event Custom|NextTextBox
  ;[1 1 1] open textbox
  (Widget|RemovefromParent (Variables|Default|GetRef_TextBox))
  (Input|SetInputModeGameandUI (Game|GetPlayerController 0) 0 "DoNotLock" true false))

(event Custom|Initialize%20Loose%20Win%20Loop
  ;[1 1 1] win or loose loop
  (Utilities|Time|SetTimerbyEvent (delegate Custom|Check%20if%20Game%20Lost%20or%20Won) 0.0167 true))

(event Custom|Check%20if%20Game%20Lost%20or%20Won
  ;[1 1 1] win or loose loop
  (if (<= (Variables|Default|GetCurrency) 0)
    ;;[1 1 1] game lost
    (Game|SetGamePaused true)
    (bind _returnvalue (UserInterface|CreateWidget "/Game/Blueprints/UI_Widgets/W_LostScreen.W_LostScreen_C"))
    (UserInterface|Viewport|AddtoViewport _returnvalue 0)
    (else
      ;;[1 1 1] game won
      (if (== (Variables|Default|GetTemples%20Found) (Variables|Default|GetTotal%20Temples))
        (bind _returnvalue_2 (UserInterface|CreateWidget "/Game/Blueprints/UI_Widgets/W_Winning_Screen.W_Winning_Screen_C"))
        (UserInterface|Viewport|AddtoViewport _returnvalue_2 0)))))

(event Custom|Initialize%20Checking%20Tutorial%20Temple
  (Utilities|Time|SetTimerbyEvent (delegate Custom|Check%20For%20First%20Temple) 0.5 true))

(event Custom|Check%20For%20First%20Temple
  (if (== (Variables|Default|GetTemples%20Found) 1)
    (Variables|Default|SetCurrent%20Text (Variables|Default|GetGo%20On%20Your%20Quest%20Please))
    (CallFunction|OpenTextbox)))

(event Custom|Open%20Textbox
  ;[1 1 1] open textbox
  (Input|SetInputModeUIOnly (Game|GetPlayerController 0) 0 "DoNotLock" false)
  (bind _returnvalue (UserInterface|CreateWidget "/Game/Blueprints/UI_Widgets/W_Textbox.W_Textbox_C"))
  (bind _output_get (Variables|Default|SetRef_TextBox _returnvalue))
  (UserInterface|Viewport|AddtoViewport _output_get 0)
  (EventDispatchers|BindEventtoOnClicked (Variables|/Game/Blueprints/UI_Widgets/W_Textbox.W_Textbox_C|GetButtonNext (Variables|Default|GetRef_TextBox)) (delegate Custom|NextTextBox)))

(event EventBeginPlay
  (bind _returnvalue (Game|GetPlayerController 0))
  ;[1 1 1] Main Menu Screen
  (bind _returnvalue_2 (UserInterface|CreateWidget "/Game/Blueprints/UI_Widgets/W_MenuScreen.W_MenuScreen_C"))
  (bind _output_get (Variables|Default|SetRef_MainScreen _returnvalue_2))
  (UserInterface|Viewport|AddtoViewport _output_get 0)
  (Game|SetGamePaused true)
  (Input|SetInputModeUIOnly _returnvalue (Variables|Default|GetRef_MainScreen) "DoNotLock" false)
  (Variables|/Script/Engine.PlayerController|SetbShowMouseCursor _returnvalue true)
  ;[1 1 1] Credit Screen
  (EventDispatchers|AssignOnClicked (Variables|/Game/Blueprints/UI_Widgets/W_MenuScreen.W_MenuScreen_C|GetButtonCredits (Variables|Default|GetRef_MainScreen)) (delegate Custom|CreditButtonClicked))
  ;[1 1 1] Start Game with Loading Screen & Delay
  (EventDispatchers|AssignOnClicked (Variables|/Game/Blueprints/UI_Widgets/W_MenuScreen.W_MenuScreen_C|GetButtonPlay (Variables|Default|GetRef_MainScreen)) (delegate Custom|Play%20Button%20Clicked)))

(event EventTick
  (params (DeltaSeconds :type Float%20%28single-precision%29))
  (bind _returnvalue (Class|WidgetLayoutLibrary|GetMousePositiononViewport))
  (bind _returnvalue_2 (Class|WidgetLayoutLibrary|GetViewportWidgetGeometry))
  (if (not (Game|IsGamePaused))
    (if (< (.X (Math|Vector2D|BreakVector2D _returnvalue)) 0.0)
      (CallFunction|MoveCam (Math|Vector|MakeVector 0.0 -25.0 0.0))
      (elif (> (.X (Math|Vector2D|BreakVector2D _returnvalue)) (- (.X (Math|Vector2D|BreakVector2D (Class|SlateBlueprintLibrary|GetLocalSize _returnvalue_2))) 5e+01))
        (CallFunction|MoveCam (Math|Vector|MakeVector 0.0 25.0 0.0))
        (elif (< (.Y (Math|Vector2D|BreakVector2D _returnvalue)) 0.0)
          (CallFunction|MoveCam (Math|Vector|MakeVector 25.0 0.0 0.0))
          (elif (> (.Y (Math|Vector2D|BreakVector2D _returnvalue)) (+ (.Y (Math|Vector2D|BreakVector2D (Class|SlateBlueprintLibrary|GetLocalSize _returnvalue_2))) 5e+01))
            (CallFunction|MoveCam (Math|Vector|MakeVector -25.0 0.0 0.0))))))))

(event Input|ActionEvents|InputActionOptionsMenu
  (params (Key :type Key%20Structure :default "None"))
  (bind _returnvalue (Game|GetPlayerController 0))
  ;[1 1 1] open pause menu
  (:Pressed
    (bind _returnvalue_2 (UserInterface|CreateWidget "/Game/Blueprints/UI_Widgets/W_PauseScreen.W_PauseScreen_C"))
    (bind _output_get (Variables|Default|SetRef_PauseScreen _returnvalue_2))
    (UserInterface|Viewport|AddtoViewport _output_get 0)
    (Input|SetInputModeUIOnly _returnvalue 0 "DoNotLock" false)
    (Variables|/Script/Engine.PlayerController|SetbShowMouseCursor _returnvalue true)
    ;[1 1 1] continue game from pause screen
    (EventDispatchers|BindEventtoOnClicked (Variables|/Game/Blueprints/UI_Widgets/W_PauseScreen.W_PauseScreen_C|GetButtonContinue (Variables|Default|GetRef_PauseScreen)) (delegate Custom|Coninue%20Game))))

(event Input|ActionEvents|InputActionTestTextbox
  (params (Key :type Key%20Structure :default "None"))
  ;[1 1 1] open textbox
  (:Pressed
    (CallFunction|OpenTextbox)))

(event Input|AxisEvents|InputAxisMoveForward
  (params (AxisValue :type Float%20%28single-precision%29))
  (if (not (Game|IsGamePaused))
    (CallFunction|MoveCam (Math|Vector|MakeVector (* AxisValue 25.0) 0.0 0.0))))

(event Input|AxisEvents|InputAxisMoveRight
  (params (AxisValue :type Float%20%28single-precision%29))
  (if (not (Game|IsGamePaused))
    (CallFunction|MoveCam (Math|Vector|MakeVector 0.0 (* AxisValue 25.0) 0.0))))

(event Input|AxisEvents|InputAxisCameraZoom
  (params (AxisValue :type Float%20%28single-precision%29))
  (bind _returnvalue (Game|Player|GetPlayerPawn 0))
  (bind _returnvalue_2 (Transformation|GetActorLocation _returnvalue))
  (if (not (Game|IsGamePaused))
    (if (and (< (.z _returnvalue_2) 5e+02) (> (.z _returnvalue_2) -1.4e+03))
      (CallFunction|MoveCam (Math|Vector|MakeVector 0.0 0.0 (* AxisValue -1e+01)))
      (elif (> (.z _returnvalue_2) 499.0)
        (CallFunction|MoveCam (Math|Vector|MakeVector 0.0 0.0 -1.0))
        (elif (< (.z _returnvalue_2) -1399.0)
          (CallFunction|MoveCam (Math|Vector|MakeVector 0.0 0.0 1.0)))))))

(event Input|KeyboardEvents|J
  (params (Key :type Key%20Structure :default "None"))
  (:Pressed
    (Variables|Default|SetCurrency (+ (Variables|Default|GetCurrency) 5))))

(fn ConstructionScript)

(fn MoveCam
  (params (B :type Vector))
  (bind _returnvalue (Pawn|GetControlledPawn))
  (Transformation|SetActorLocation _returnvalue (+ (Transformation|GetActorLocation _returnvalue) B) false false))