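; BP_Tree is a Blueprint that, despite its name, runs the game's UI flow: main menu, credits, HUD, pause screen and textbox.
; BeginPlay shows the main menu with the game paused; Play clears all widgets, unpauses and adds the HUD.
; Input actions open the pause screen, which switches to UI-only input without pausing, and a test textbox.
; Button clicks are bound here to custom events that open or close widgets.
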(event Custom|CreditButtonClicked
  ;[1 1 1] Credit Screen
  (bind _returnvalue (UserInterface|CreateWidget "/Game/Blueprints/UI_Widgets/W_CreditsScreen.W_CreditsScreen_C"))
  (UserInterface|Viewport|AddtoViewport _returnvalue 0))

(event Custom|Play%20Button%20Clicked
  ;[1 1 1] Start Game
  (Viewport|RemoveAllWidgets)
  (Input|SetInputModeGameOnly (Game|GetPlayerController 0) false)
  (Game|SetGamePaused false)
  (bind _returnvalue (UserInterface|CreateWidget "/Game/Blueprints/UI_Widgets/W_HUD.W_HUD_C"))
  (UserInterface|Viewport|AddtoViewport _returnvalue 0))

(event Custom|Coninue%20Game
  ;[1 1 1] continue game from pause screen
  (Widget|RemovefromParent (Variables|Default|GetRef_PauseMenu))
  (Input|SetInputModeGameOnly (Game|GetPlayerController 0) false)
  (Game|SetGamePaused false))

(event Custom|Next%20Textbox
  (Widget|RemovefromParent (Variables|Default|GetRef_Textbox)))

(event EventBeginPlay
  (bind _returnvalue (Game|GetPlayerController 0))
  ;[1 1 1] Main Menu Screen
  (bind _returnvalue_2 (UserInterface|CreateWidget "/Game/Blueprints/UI_Widgets/W_MenuScreen.W_MenuScreen_C"))
  (bind _output_get (Variables|Default|SetRef_MainMenu _returnvalue_2))
  (UserInterface|Viewport|AddtoViewport _output_get 0)
  (Game|SetGamePaused true)
  (Input|SetInputModeUIOnly _returnvalue (Variables|Default|GetRef_MainMenu) "DoNotLock" false)
  (Variables|/Script/Engine.PlayerController|SetbShowMouseCursor _returnvalue true)
  ;[1 1 1] Credit Screen
  (EventDispatchers|AssignOnClicked (Variables|/Game/Blueprints/UI_Widgets/W_MenuScreen.W_MenuScreen_C|GetButtonCredits (Variables|Default|GetRef_MainMenu)) (delegate Custom|CreditButtonClicked))
  ;[1 1 1] Start Game
  (EventDispatchers|AssignOnClicked (Variables|/Game/Blueprints/UI_Widgets/W_MenuScreen.W_MenuScreen_C|GetButtonPlay (Variables|Default|GetRef_MainMenu)) (delegate Custom|Play%20Button%20Clicked)))

(event Input|ActionEvents|InputActionOptionsMenu
  (params (Key :type Key%20Structure :default "None"))
  (bind _returnvalue (Game|GetPlayerController 0))
  ;[1 1 1] open pause menu
  (:Pressed
    (bind _returnvalue_2 (UserInterface|CreateWidget "/Game/Blueprints/UI_Widgets/W_PauseScreen.W_PauseScreen_C"))
    (bind _output_get (Variables|Default|SetRef_PauseMenu _returnvalue_2))
    (UserInterface|Viewport|AddtoViewport _output_get 0)
    (Input|SetInputModeUIOnly _returnvalue 0 "DoNotLock" false)
    (Variables|/Script/Engine.PlayerController|SetbShowMouseCursor _returnvalue true)
    ;[1 1 1] continue game from pause screen
    (EventDispatchers|BindEventtoOnClicked (Variables|/Game/Blueprints/UI_Widgets/W_PauseScreen.W_PauseScreen_C|GetButtonContinue (Variables|Default|GetRef_PauseMenu)) (delegate Custom|Coninue%20Game))))

(event Input|ActionEvents|InputActionTest_Textbox
  (params (Key :type Key%20Structure :default "None"))
  (:Pressed
    (bind _returnvalue (UserInterface|CreateWidget "/Game/Blueprints/UI_Widgets/W_Textbox.W_Textbox_C"))
    (bind _output_get (Variables|Default|SetRef_Textbox _returnvalue))
    (UserInterface|Viewport|AddtoViewport _output_get 0)
    (EventDispatchers|AssignOnClicked (Variables|/Game/Blueprints/UI_Widgets/W_Textbox.W_Textbox_C|GetButton_Next (Variables|Default|GetRef_Textbox)) (delegate Custom|Next%20Textbox))))

(fn ConstructionScript)